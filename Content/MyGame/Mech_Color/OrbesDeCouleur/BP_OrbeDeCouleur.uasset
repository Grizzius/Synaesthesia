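; Interactable color orb pickup that unlocks its assigned color (blue, red or yellow) in the game.
; On interact, if GI_Main does not already have that color unlocked, it unlocks it and shows the matching unlock widget.
; It then activates an effect, hides the sphere, disables its collision and destroys itself after a short delay.
; The construction script sets the sphere material from the color, and interact HUD events toggle a prompt widget.
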(event EventBeginPlay)

(event Collision|EventActorBeginOverlap
  (params (OtherActor :type Actor%20Object%20Reference)))

(event EventTick
  (params (DeltaSeconds :type Float%20%28single-precision%29)))

(event EventOnInteract
  (params (Player%20Ref :type BP%20First%20Person%20Object%20Reference))
  (bind _color (Variables|Default|GetColor))
  (bind _asgi_main (Utilities|Casting|CastToGI_Main (Game|GetGameInstance)))
  (if (not (Utilities|Array|Get(acopy) (Variables|/Game/MyGame/Data/GameInstance/GI_Main.GI_Main_C|GetUnlockedColor _asgi_main) (Math|Conversions|ToInteger(Byte) (Variables|Default|GetColor))))
    (Default|EventUnlockColor _asgi_main (Math|Conversions|ToInteger(Byte) _color))
    (bind _returnvalue (UserInterface|CreateWidget (Utilities|Select :Index _color :NewEnumerator0 "/Game/MyGame/UI_HUD/WB_Tutos/BlueUnlock.BlueUnlock_C" :NewEnumerator1 "/Game/MyGame/UI_HUD/WB_Tutos/RedUnlock.RedUnlock_C" :NewEnumerator2 "/Game/MyGame/UI_HUD/WB_Tutos/YellowUnlock.YellowUnlock_C" :NewEnumerator4 0)))
    (UserInterface|Viewport|AddtoViewport _returnvalue 0)
    (Components|Activation|Activate (Variables|Default|GetFxNia_Blue) false)
    (Rendering|SetVisibility (Variables|Default|GetSphere) false false)
    (Collision|SetCollisionEnabled (Variables|Default|GetSphere) "NoCollision")
    (Utilities|FlowControl|Delay 2.0)
    (Actor|DestroyActor)))

(event EventDisplayInteractHUD
  (Rendering|SetVisibility (Variables|Default|GetWidget) true false))

(event EventHideInteractHUD
  (Rendering|SetVisibility (Variables|Default|GetWidget) false false))

(fn ConstructionScript
  (Rendering|Material|SetMaterial (Variables|Default|GetSphere) 0 (Utilities|Select :Index (Variables|Default|GetColor) :NewEnumerator0 "/Game/MyGame/Mech_Color/Materials/Mat_Blue.Mat_Blue" :NewEnumerator1 "/Game/MyGame/Mech_Color/Materials/Mat_Red.Mat_Red" :NewEnumerator2 "/Game/MyGame/Mech_Color/Materials/Mat_Yellow.Mat_Yellow" :NewEnumerator4 "/Game/UE5/FPWeapon/Materials/BaseMaterial.BaseMaterial")))