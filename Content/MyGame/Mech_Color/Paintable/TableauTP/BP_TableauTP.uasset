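; BP_TableauTP is a paintable painting that teleports "canTP" actors to another painting of the same color.
; Color changes update the frame material and timestamp, and a third same-colored painting resets the oldest to None.
; Box overlaps, except held cubes, move the actor to the partner's TPPoint, pass on its color, redirect momentum and turn the player's view.
; Both paintings take a brief cooldown to prevent bounce-back; ToggleParticle is an empty stub.
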(event OnComponentBeginOverlap(BoxColision)
  (params (OverlappedComponent :type Primitive%20Component%20Object%20Reference) (OtherActor :type Actor%20Object%20Reference) (OtherComp :type Primitive%20Component%20Object%20Reference) (OtherBodyIndex :type Integer) (bFromSweep :type Boolean) (SweepResult :type Hit%20Result%20Structure%20%28by%20ref%29))
  (bind _asbp_paintable_cube (Utilities|Casting|CastToBP_PaintableCube OtherActor)
    (:then
      (bind _is_held_item (Default|IsHeldItem? _asbp_paintable_cube))
      (if (not _is_held_item)
        (if (Math|Boolean|ANDBoolean (Actor|ActorHasTag OtherActor "canTP") (Variables|Default|GetbCanTP) (Utilities|Enum|NotEqual(Enum) (Variables|Default|GetColor) "NewEnumerator4")) :!label _label
          (bind _otherpainting (CallFunction|FindOtherPainting))
          (Utilities|IsValid _otherpainting
            (:Is%20Valid
              (CallFunction|EventTPCooldown _otherpainting)
              (CallFunction|EventTPCooldown)
              (Transformation|SetActorLocationAndRotation OtherActor (Transformation|GetWorldLocation (Variables|BP_TableauTP_C|GetTP%20Point _otherpainting)) (Math|Rotator|MakeRotator 0.0 0.0 (.yaw (Transformation|GetWorldRotation (Variables|BP_TableauTP_C|GetTP%20Point _otherpainting)))) false true)
              (Class|BPICanTP|AddImpulseonTP(Message) OtherActor (* (Math|Vector|GetForwardVector (Variables|BP_TableauTP_C|GetArrow _otherpainting)) (Math|Vector|VectorLength (Transformation|GetVelocity OtherActor)) 1.0))
              (Class|BPIPaintable|ChangeColor(Message) OtherActor (Variables|Default|GetColor))
              (bind _asbp_first_person (Utilities|Casting|CastToBP_FirstPerson OtherActor))
              (Pawn|SetControlRotation (Pawn|GetController _asbp_first_person) (Math|Rotator|MakeRotator 0.0 0.0 (.yaw (Transformation|GetWorldRotation (Variables|BP_TableauTP_C|GetArrow _otherpainting))))))))))
    (:CastFailed
      (goto _label))))

(event Custom|EventTPCooldown
  (Variables|Default|SetbCanTP false)
  (Utilities|FlowControl|Delay 0.2)
  (Variables|Default|SetbCanTP true))

(event Custom|EventChangeColor
  (params (New%20Color :type EnumColor%20Enum :default "NewEnumerator0"))
  (if (not (Utilities|Enum|Equal(Enum) New%20Color (Variables|Default|GetColor)))
    (CallFunction|UpdateMaterial New%20Color)))

(event EventBeginPlay
  (Utilities|FlowControl|Delay 1.0)
  (if (Utilities|Enum|NotEqual(Enum) (Variables|Default|GetColor) "NewEnumerator4")
    (Variables|Default|SetBeginPlayBool true)
    (bind _output_get (Variables|Default|SetTemporaryColor (Variables|Default|GetColor)))
    (CallFunction|ChangeColor "NewEnumerator4")
    (Variables|Default|SetBeginPlayBool false)
    (CallFunction|ChangeColor _output_get)))

(event Collision|EventActorBeginOverlap
  (params (OtherActor :type Actor%20Object%20Reference)))

(event EventOnInteract
  (params (Player%20Ref :type BP%20First%20Person%20Object%20Reference)))

(event EventChangeColor
  (params (newColor :type EnumColor%20Enum :default "NewEnumerator0"))
  (CallFunction|EventChangeColor newColor))

(event EventTick
  (params (DeltaSeconds :type Float%20%28single-precision%29)))

(fn ConstructionScript
  (CallFunction|UpdateMaterial (Variables|Default|GetColor)))

(fn UpdateMaterial
  (params (NewParam :type EnumColor%20Enum :default "NewEnumerator0"))
  (bind _otherpainting (CallFunction|FindOtherPainting))
  (Utilities|IsValid _otherpainting
    (:Is%20Valid
      (CallFunction|ToggleParticle _otherpainting false))
    (:Is%20Not%20Valid
      _))
  (Variables|Default|SetColor NewParam)
  (Rendering|Material|SetMaterial (Variables|Default|Getcadretp) 0 (Utilities|Select :Index (Variables|Default|GetColor) :NewEnumerator0 "/Game/MyGame/3D_Assets/Cadre_TP/MI_CadreTPBleu.MI_CadreTPBleu" :NewEnumerator1 "/Game/MyGame/3D_Assets/Cadre_TP/MI_CadreTPRouge.MI_CadreTPRouge" :NewEnumerator2 "/Game/MyGame/3D_Assets/Cadre_TP/MI_CadreTPJaune.MI_CadreTPJaune" :NewEnumerator4 "/Game/MyGame/3D_Assets/Cadre_TP/MI_CadreTPBlanc.MI_CadreTPBlanc"))
  (CallFunction|OnChangeColor))

(fn OnChangeColor
  (Variables|Default|SetColorTime (Utilities|Time|GetTimeSeconds))
  (if (not (Variables|Default|GetBeginPlayBool))
    (CallFunction|EraseLastTableau)
    (if (Utilities|Enum|NotEqual(Enum) (Variables|Default|GetColor) "NewEnumerator4")
      (bind _otherpainting (CallFunction|FindOtherPainting))
      (Utilities|IsValid _otherpainting
        (:Is%20Valid
          (CallFunction|ToggleParticle _otherpainting true)
          (CallFunction|ToggleParticle true))
        (:Is%20Not%20Valid
          (CallFunction|ToggleParticle false :!label _label)))
      (else
        (goto _label)))))

(fn SpawnCube
  (params (Cube :type BP%20Paintable%20Cube%20Object%20Reference))
  (bind _tp_point (Variables|Default|GetTP%20Point))
  (switch Utilities|FlowControl|Switch|SwitchonEnumColor (Variables|Default|GetColor)
    (:NewEnumerator0
      (bind _outactors (Actor|GetAllActorsOfClass "/Game/MyGame/Mech_Color/Paintable/TableauTP/BP_DataTableau.BP_DataTableau_C"))
      (for _array_element 0
        (if (!= _array_element self)
          (Variables|BP_TableauTP_C|SetWillSpawn? _array_element true)
          (Transformation|SetWorldLocationAndRotation (Variables|/Script/Engine.Actor|GetRootComponent Cube) (Transformation|GetWorldLocation _tp_point) (Transformation|GetWorldRotation _tp_point) false true))))))

(fn EraseLastTableau
  (bind _same_colored_paintings (CallFunction|FindAllPaintingsOfSameColor))
  (if (> (Utilities|Array|Length _same_colored_paintings) 2)
    (for _array_element _same_colored_paintings
      (Utilities|IsValid _array_element
        (:Is%20Valid
          (Utilities|Array|Add (LocalVariables|GetL_PaintingTimes) (Variables|BP_TableauTP_C|GetColorTime _array_element)))))
    (for (_array_element_2 _array_index) _same_colored_paintings
      (Utilities|IsValid _array_element_2
        (:Is%20Valid
          (if (== _array_index (.IndexOfMinValue (Math|Float|MinOfFloatArray (LocalVariables|GetL_PaintingTimes))))
            (CallFunction|EventChangeColor _array_element_2 "NewEnumerator4")
            (CallFunction|ToggleParticle _array_element_2 false)))))))

(fn FindOtherPainting
  (bind _outactors (Actor|GetAllActorsOfClass "BP_TableauTP_C"))
  (bind _array_element (Utilities|Array|ForEachLoopwithBreak _outactors)
    (:LoopBody
      (if (and (Utilities|Enum|Equal(Enum) (Variables|BP_TableauTP_C|GetColor _array_element) (Variables|Default|GetColor)) (not (== _array_element self)))
        (LocalVariables|SetNewLocalVar _array_element)))
    (:Completed
      (return (LocalVariables|GetNewLocalVar)))))

(fn FindAllPaintingsOfSameColor
  (bind _outactors (Actor|GetAllActorsOfClass "BP_TableauTP_C"))
  (for _array_element _outactors
    (if (Utilities|Enum|Equal(Enum) (Variables|Default|GetColor) (Variables|BP_TableauTP_C|GetColor _array_element))
      (Utilities|Array|Add (LocalVariables|GetL_SameColoredPaintings) _array_element)))
  (return (LocalVariables|GetL_SameColoredPaintings)))

(fn ToggleParticle
  (params (isActive :type Boolean)))