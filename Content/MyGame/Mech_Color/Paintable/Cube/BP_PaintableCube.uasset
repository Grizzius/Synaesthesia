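; A physics crate that the player can paint, pick up and drop, with behavior set by its color.
; ChangeColor swaps material and resets physics; Blue floats upward, Yellow bounces and launches the player, Red weighs less when hit.
; A player hit on a Red cube opens a timeline window in which it shatters other paintable cubes it strikes.
; GroCube variants stop simulating physics, and conveyor tagging happens at BeginPlay.
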(event OnComponentHit(StaticMesh)
  (params (HitComponent :type Primitive%20Component%20Object%20Reference) (OtherActor :type Actor%20Object%20Reference) (OtherComp :type Primitive%20Component%20Object%20Reference) (NormalImpulse :type Vector :default "0, 0, 0") (Hit :type Hit%20Result%20Structure%20%28by%20ref%29))
  (Utilities|FlowControl|Sequence
    (:then_0
      (if (== OtherActor (Game|GetPlayerCharacter 0))
        (if (Utilities|Enum|Equal(Enum) (Variables|Default|GetColor) "NewEnumerator1")
          (Game|Feedback|PlayDynamicForceFeedback (Game|GetPlayerController 0) 0.2 0.2 true true true true)
          (Utilities|FlowControl|Sequence
            (:then_0
              (Utilities|FlowControl|DoOnce false :!label _label
                (:Completed
                  (Audio|PlaySoundatLocation "/Game/MyGame/Joueur/Gun/Sound/PaintSound/SFX_RedPaint.SFX_RedPaint" (Transformation|GetActorLocation) "0, 0, 0" 1.0 1.0 0.0 0 0 0 0)
                  (Utilities|FlowControl|Delay 0.2)
                  (goto _label Reset))))
            (:then_1
              (Utilities|FlowControl|Sequence
                (:then_0
                  (Class|PrimitiveComponent|SetLinearDamping (Variables|Default|GetStaticMesh) 0.1)
                  (Utilities|FlowControl|Delay 1.0)
                  (Class|PrimitiveComponent|SetLinearDamping (Variables|Default|GetStaticMesh) 0.01))
                (:then_1
                  (Timeline|Timeline_1 PlayFromStart
                    (:Update
                      (Variables|Red|SetbCanDestroyCube true))
                    (:Finished
                      (Variables|Red|SetbCanDestroyCube false))))))))))
    (:then_1
      ;[1 1 1] Si le cube est rouge, détruit l'autre cube
      (if (Utilities|Enum|Equal(Enum) (Variables|Default|GetColor) "NewEnumerator1")
        (bind _asbp_paintable_cube (Utilities|Casting|CastToBP_PaintableCube OtherActor))
        (if (Variables|Red|GetbCanDestroyCube)
          (Audio|PlaySoundatLocation "/Game/MyGame/Joueur/Gun/Sound/PaintSound/SFX_RedCubeDestroy.SFX_RedCubeDestroy" (Transformation|GetActorLocation _asbp_paintable_cube) "0, 0, 0" 1.0 1.0 0.0 0 0 0 0)
          (Physics|AddImpulse (Variables|Default|GetStaticMesh) (* (Math|Vector|GetUnitDirection(Vector) (Transformation|GetActorLocation) (Transformation|GetActorLocation _asbp_paintable_cube)) (Math|Conversions|ToVector(Float) -2e+02)) "None" true)
          (Game|SpawnActorfromClass "/Game/MyGame/Mech_Color/Paintable/Cube/BP_CubeDestroy_GeometryCollection_Blueprint1.BP_CubeDestroy_GeometryCollection_Blueprint1_C" (Math|Transform|MakeTransform (.location (Transformation|GetActorTransform _asbp_paintable_cube)) (.rotation (Transformation|GetActorTransform _asbp_paintable_cube)) (Math|Vector|MakeVector (.x (Math|Vector|ClampVectorSize (Math|Vector|MakeVector (.x (.scale (Transformation|GetActorTransform _asbp_paintable_cube))) (.y (.scale (Transformation|GetActorTransform _asbp_paintable_cube))) (.z (.scale (Transformation|GetActorTransform _asbp_paintable_cube)))) 0.0 5.0)) (.y (Math|Vector|ClampVectorSize (Math|Vector|MakeVector (.x (.scale (Transformation|GetActorTransform _asbp_paintable_cube))) (.y (.scale (Transformation|GetActorTransform _asbp_paintable_cube))) (.z (.scale (Transformation|GetActorTransform _asbp_paintable_cube)))) 0.0 5.0)) (.z (Math|Vector|ClampVectorSize (Math|Vector|MakeVector (.x (.scale (Transformation|GetActorTransform _asbp_paintable_cube))) (.y (.scale (Transformation|GetActorTransform _asbp_paintable_cube))) (.z (.scale (Transformation|GetActorTransform _asbp_paintable_cube)))) 0.0 5.0)))) "Undefined" 0 (Utilities|Select :Index (Variables|BP_PaintableCube_C|GetColor _asbp_paintable_cube) :NewEnumerator0 "/Game/MyGame/3D_Assets/box/MTI_CaisseBleu.MTI_CaisseBleu" :NewEnumerator1 "/Game/MyGame/3D_Assets/box/MTI_CaisseRouge.MTI_CaisseRouge" :NewEnumerator2 "/Game/MyGame/3D_Assets/box/MTI_CaisseJaune.MTI_CaisseJaune" :NewEnumerator4 "/Game/MyGame/3D_Assets/box/MTI_CaisseBlanc.MTI_CaisseBlanc") 0)
          (Game|SpawnActorfromClass "/Game/MyGame/Mech_Color/Paintable/Cube/Bp_ExploCube.Bp_ExploCube_C" (Math|Transform|MakeTransform (.location (Transformation|GetActorTransform _asbp_paintable_cube)) (.rotation (Transformation|GetActorTransform _asbp_paintable_cube)) (Math|Vector|MakeVector (.x (Math|Vector|ClampVectorSize (Math|Vector|MakeVector (.x (.scale (Transformation|GetActorTransform _asbp_paintable_cube))) (.y (.scale (Transformation|GetActorTransform _asbp_paintable_cube))) (.z (.scale (Transformation|GetActorTransform _asbp_paintable_cube)))) 0.0 5.0)) (.y (Math|Vector|ClampVectorSize (Math|Vector|MakeVector (.x (.scale (Transformation|GetActorTransform _asbp_paintable_cube))) (.y (.scale (Transformation|GetActorTransform _asbp_paintable_cube))) (.z (.scale (Transformation|GetActorTransform _asbp_paintable_cube)))) 0.0 5.0)) (.z (Math|Vector|ClampVectorSize (Math|Vector|MakeVector (.x (.scale (Transformation|GetActorTransform _asbp_paintable_cube))) (.y (.scale (Transformation|GetActorTransform _asbp_paintable_cube))) (.z (.scale (Transformation|GetActorTransform _asbp_paintable_cube)))) 0.0 5.0)))) "Undefined" 0 0)
          (Actor|DestroyActor _asbp_paintable_cube))))))

(event Custom|OnChangeColor
  (bind _returnvalue (Transformation|GetVelocity))
  (CallFunction|ResetColor)
  (switch Utilities|FlowControl|Switch|SwitchonEnumColor (Variables|Default|GetColor)
    (:NewEnumerator0
      (Physics|SetEnableGravity (Variables|Default|GetStaticMesh) false)
      (for _array_element (Collision|GetOverlappingActors "/Game/MyGame/Joueur/Character/BP_FirstPerson.BP_FirstPerson_C" :!class /Script/Engine.Actor)
        (Utilities|IsValid _array_element
          (:Is%20Valid
            (Physics|SetSimulatePhysics (Variables|Default|GetStaticMesh) false))))
      (Physics|SetPhysicsLinearVelocity (Variables|Default|GetStaticMesh) (Math|Vector|MakeVector (.x _returnvalue) (.y _returnvalue) 0.0) false "None"))
    (:NewEnumerator2
      (CallFunction|SetPhysicsMaterial "/Game/MyGame/Mech_Color/Paintable/Cube/BouncyCrate.BouncyCrate"))))

(event Custom|UpdateScale
  (params (ReduceSize :type Boolean))
  (if ReduceSize
    (bind _newtrack_0 (Timeline|TL_ChangeScale ReverseFromEnd)
      (:Update
        (Transformation|SetWorldScale3D (Variables|Default|GetStaticMesh) (Math|Vector|Lerp(Vector) "0.700000,0.700000,0.700000" "1.000000,1.000000,1.000000" _newtrack_0))))
    (else
      (Timeline|TL_ChangeScale PlayFromStart))))

(event EventTick
  (params (DeltaSeconds :type Float%20%28single-precision%29))
  (bind _returnvalue (* DeltaSeconds "0.000000,0.000000,200.000000"))
  (bind _staticmesh (Variables|Default|GetStaticMesh))
  (Utilities|FlowControl|Sequence
    (:then_0
      (switch Utilities|FlowControl|Switch|SwitchonEnumColor (Variables|Default|GetColor)
        (:NewEnumerator0
          (if (Physics|IsSimulatingPhysics (Variables|Default|GetStaticMesh) "None")
            (Physics|AddForce _staticmesh (* _returnvalue 4e+01) "None" true)
            (else
              (Transformation|AddWorldOffset _staticmesh _returnvalue true false))))))
    (:then_1
      (if (< (.z (Transformation|GetActorLocation)) -1.5e+04)
        (Actor|DestroyActor)))))

(event EventBeginPlay
  (Utilities|FlowControl|Sequence
    (:then_0
      ;[1 1 1] Ajoute le tag pour se faire bouger par le tapis roulant
      (bind _output_get (Variables|Default|SetTags (Variables|Actor|GetTags)))
      (bind _asgi_main (Utilities|Casting|CastToGI_Main (Game|GetGameInstance)))
      (Utilities|Array|AddUnique _output_get (Variables|/Game/MyGame/Data/GameInstance/GI_Main.GI_Main_C|GetTagNameTapisRoulant _asgi_main)))
    (:then_1
      (CallFunction|OnChangeColor)
      (Variables|Default|SetstartPosition (Transformation|GetActorLocation))
      (Variables|Default|SetstartScale (Transformation|GetActorScale3D)))
    (:then_2
      (if (Variables|Default|GetGroCube?)
        (Physics|SetSimulatePhysics (Variables|Default|GetStaticMesh) false)))))

(event EventOnInteract
  (params (Player%20Ref :type BP%20First%20Person%20Object%20Reference))
  (bind _staticmesh (Variables|Default|GetStaticMesh))
  (if (not (Variables|Default|GetbNotPickable))
    (Variables|Interaction|SetbIsPickedUp true)
    (Variables|/Game/MyGame/Joueur/Character/BP_FirstPerson.BP_FirstPerson_C|SetHeldItem Player%20Ref self)
    (CallFunction|UpdateMaterial (Variables|Default|GetColor))
    (CallFunction|UpdateScale true)
    (Collision|SetCollisionResponsetoChannel (Variables|Default|GetStaticMesh) "ECC_Pawn" "ECR_Ignore")
    (Physics|SetEnableGravity _staticmesh false)
    (Physics|SetSimulatePhysics _staticmesh false)))

(event Collision|EventHit
  (params (MyComp :type Primitive%20Component%20Object%20Reference) (Other :type Actor%20Object%20Reference) (OtherComp :type Primitive%20Component%20Object%20Reference) (bSelfMoved :type Boolean) (HitLocation :type Vector :default "0, 0, 0") (HitNormal :type Vector :default "0, 0, 0") (NormalImpulse :type Vector :default "0, 0, 0") (Hit :type Hit%20Result%20Structure%20%28by%20ref%29))
  (switch Utilities|FlowControl|Switch|SwitchonEnumColor (Variables|Default|GetColor)
    (:NewEnumerator0
      (CallFunction|ChangeMass 1e+02)
      (Utilities|Casting|CastToBP_FirstPerson Other)
      (Physics|SetSimulatePhysics (Variables|Default|GetStaticMesh) false))
    (:NewEnumerator1
      (Utilities|IsValid Other
        (:Is%20Valid
          (if (not (Actor|ActorHasTag Other "CantPushRedCube"))
            (if (Variables|Default|GetGroCube?)
              (Physics|SetSimulatePhysics (Variables|Default|GetStaticMesh) false)
              (else
                (CallFunction|ChangeMass 1e+01)))))))
    (:NewEnumerator2
      (CallFunction|ChangeMass 1e+02)
      (bind _asbp_first_person (Utilities|Casting|CastToBP_FirstPerson Other))
      (Character|LaunchCharacter _asbp_first_person (Math|Vector|MakeVector 0.0 0.0 (* (Math|Float|Clamp(Float) (Math|Vector|VectorLength (Transformation|GetComponentVelocity (Variables|/Script/Engine.Actor|GetRootComponent _asbp_first_person))) 4.2e+02 4.2e+03) 0.9)) false true))
    (:NewEnumerator4
      (if (Variables|Default|GetGroCube?)
        (Physics|SetSimulatePhysics (Variables|Default|GetStaticMesh) false)
        (else
          (CallFunction|ChangeMass 1e+02))))))

(event EventDisplayInteractHUD
  (if (not (Variables|Default|GetbNotPickable))
    (Rendering|SetVisibility (Variables|Default|GetWidget) true false)))

(event EventHideInteractHUD
  (Rendering|SetVisibility (Variables|Default|GetWidget) false false))

(event EventAddImpulseonTP
  (params (Impulse :type Vector :default "0, 0, 0"))
  (Physics|AddImpulse (Variables|Default|GetStaticMesh) (select (Variables|Interaction|GetbIsPickedUp) "0, 0, 0" Impulse) "None" true))

(event Collision|EventActorEndOverlap
  (params (OtherActor :type Actor%20Object%20Reference))
  (switch Utilities|FlowControl|Switch|SwitchonEnumColor (Variables|Default|GetColor)
    (:NewEnumerator0
      (Physics|SetSimulatePhysics (Variables|Default|GetStaticMesh) true))))

(event EventDrop
  (bind _staticmesh (Variables|Default|GetStaticMesh))
  (bind _asbp_first_person (Utilities|Casting|CastToBP_FirstPerson (Game|Player|GetPlayerPawn 0))
    (:then
      (Variables|/Game/MyGame/Joueur/Character/BP_FirstPerson.BP_FirstPerson_C|SetHeldItem _asbp_first_person 0))
    (:CastFailed
      _))
  (Variables|Interaction|SetbIsPickedUp false)
  (CallFunction|UpdateMaterial (Variables|Default|GetColor))
  (CallFunction|UpdateScale false)
  (Collision|SetCollisionResponsetoChannel (Variables|Default|GetStaticMesh) "ECC_Pawn" "ECR_Block")
  (Physics|SetEnableGravity (Variables|Default|GetStaticMesh) (Utilities|Select :Index (Variables|Default|GetColor) :NewEnumerator0 false :NewEnumerator1 true :NewEnumerator2 true :NewEnumerator4 true))
  (Transformation|SetActorLocation (Transformation|GetActorLocation) false true)
  (Physics|SetPhysicsLinearVelocity _staticmesh "0, 0, 0" false "None")
  (Physics|SetSimulatePhysics _staticmesh true))

(event EventChangeColor
  (params (newColor :type EnumColor%20Enum :default "NewEnumerator0"))
  (if (not (Variables|Interaction|GetbIsPickedUp))
    (CallFunction|UpdateMaterial newColor)
    (CallFunction|OnChangeColor)
    (Audio|PlaySoundatLocation (Utilities|Select :Index (Variables|Default|GetColor) :NewEnumerator0 "/Game/MyGame/Joueur/Gun/Sound/PaintSound/SFX_PaintBlue.SFX_PaintBlue" :NewEnumerator1 "/Game/MyGame/Joueur/Gun/Sound/PaintSound/SFX_RedPaint.SFX_RedPaint" :NewEnumerator2 "/Game/MyGame/Joueur/Gun/Sound/PaintSound/SFX_PaintYellow.SFX_PaintYellow" :NewEnumerator4 0) (Transformation|GetActorLocation) "0, 0, 0" 1.0 1.0 0.0 0 0 0 0)))

(fn ConstructionScript
  (CallFunction|UpdateMaterial (Variables|Default|GetColor)))

(fn UpdateMaterial
  (params (ColorInput :type EnumColor%20Enum :default "NewEnumerator0"))
  (Variables|Default|SetColor ColorInput)
  (Rendering|Material|SetMaterial (Variables|Default|GetStaticMesh) 0 (Utilities|Array|Get(acopy) (select (Variables|Interaction|GetbIsPickedUp) (Variables|Default|GetColorTextures_Grabbed) (Variables|Default|GetColorTextures)) (Math|Conversions|ToInteger(Byte) (Variables|Default|GetColor)))))

(fn SetPhysicsMaterial
  (params (new%20Physical%20Material :type Physical%20Material%20Object%20Reference))
  (Class|PrimitiveComponent|SetPhysMaterialOverride (Variables|Default|GetStaticMesh) new%20Physical%20Material))

(fn ResetColor
  (bind _staticmesh (Variables|Default|GetStaticMesh))
  (CallFunction|SetPhysicsMaterial "/Game/MyGame/Mech_Color/Paintable/Cube/DefaultPhysic.DefaultPhysic")
  (Collision|SetCollisionEnabled _staticmesh "QueryAndPhysics")
  (Physics|SetSimulatePhysics _staticmesh true)
  (Physics|SetEnableGravity _staticmesh true)
  (Physics|AddImpulse (Variables|Default|GetStaticMesh) "0.000000,0.000000,10.000000" "None" true))

(fn NewFunction0
  (params (other :type Actor%20Object%20Reference) (Hit%20Impulse :type Vector))
  (bind _ascharacter (Utilities|Casting|CastToCharacter other)
    (:then
      (LocalVariables|SetNewLocalVar_0 (Transformation|GetActorForwardVector _ascharacter)))
    (:CastFailed
      (LocalVariables|SetNewLocalVar_0 (Math|Vector|Normalize Hit%20Impulse))))
  (return (LocalVariables|GetNewLocalVar_0)))

(fn ChangeMass
  (params (Poids :type Float%20%28double-precision%29))
  (Class|PrimitiveComponent|SetMassOverrideinKg (Variables|Default|GetStaticMesh) "None" Poids true))

(fn IsHeldItem?
  (bind _asbp_first_person (Utilities|Casting|CastToBP_FirstPerson (Game|GetPlayerCharacter 0)))
  (return (== (Variables|/Game/MyGame/Joueur/Character/BP_FirstPerson.BP_FirstPerson_C|GetHeldItem _asbp_first_person) self)))