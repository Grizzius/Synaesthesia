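; Cube spawner that creates a colored, scaled BP_PaintableCube at an offset from itself and plays a spawn sound.
; At BeginPlay it binds to an existing cube's destruction or optionally spawns a new one.
; When Action's trigger count matches the required count, it destroys the current cube after a short delay, or spawns one if none exists.
; Destruction events drive respawning, gated by that same trigger check.
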(event Custom|SpawnCube
  (bind _returnvalue (Game|SpawnActorfromClass "/Game/MyGame/Mech_Color/Paintable/Cube/BP_PaintableCube.BP_PaintableCube_C" (Math|Transform|MakeTransform (+ (Transformation|GetActorLocation) (Variables|SpawnParameter|GetSpawnPoint)) (Transformation|GetActorRotation) (Variables|SpawnParameter|GetCubeScale)) "Undefined" 0 (Variables|SpawnParameter|GetCubeColor) 0))
  (bind _output_get (Variables|SpawnParameter|SetCubeReference _returnvalue))
  (Game|BindEventtoOnDestroyed _output_get (EventDispatchers|CreateEvent :!event Custom|OnCubeDestroyed))
  (Audio|PlaySoundatLocation "/Game/MyGame/Sound/SoundEffect/SFX_SpawnCube.SFX_SpawnCube" (Transformation|GetActorLocation) "0, 0, 0" 1.0 1.0 0.0 0 0 0 0))

(event Custom|OnCubeDestroyed
  (params (DestroyedActor :type Actor%20Object%20Reference))
  (if (== (Variables|Default|GetcurrentTrigger) (Variables|Default|GettriggerCount))
    (CallFunction|SpawnCube)))

(event EventBeginPlay
  (CallFunction|BeginFunction)
  (Utilities|IsValid (Variables|SpawnParameter|GetCubeReference)
    (:Is%20Valid
      (Game|BindEventtoOnDestroyed (Variables|SpawnParameter|GetCubeReference) (EventDispatchers|CreateEvent :!event Custom|OnCubeDestroyed)))
    (:Is%20Not%20Valid
      (if (Variables|SpawnParameter|GetbSpawnOnBeginPlay)
        (CallFunction|SpawnCube)))))

(event EventAction
  (params (currentTrigger :type Integer))
  (bind _cubereference (Variables|SpawnParameter|GetCubeReference))
  (if (== currentTrigger (Variables|Default|GettriggerCount))
    (Utilities|FlowControl|Delay 0.2)
    (Utilities|IsValid _cubereference
      (:Is%20Valid
        (Actor|DestroyActor _cubereference))
      (:Is%20Not%20Valid
        (CallFunction|SpawnCube)))))

(fn ConstructionScript)