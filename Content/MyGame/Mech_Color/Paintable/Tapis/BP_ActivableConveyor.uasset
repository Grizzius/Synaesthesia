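; Paintable conveyor belt that carries tagged cubes and the player while its trigger count is met.
; Paint color swaps materials and sounds and sets speed: blue reverses, red scales it by RedPush, yellow also bounces the player on hit.
; Tick moves actors in top and bottom overlap boxes in opposite directions, offsetting cubes and impulsing the player.
; On exit, CanPropulse launches physics cubes; otherwise the player's velocity is zeroed after a short delay.
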(event OnComponentHit(StaticMesh)
  (params (HitComponent :type Primitive%20Component%20Object%20Reference) (OtherActor :type Actor%20Object%20Reference) (OtherComp :type Primitive%20Component%20Object%20Reference) (NormalImpulse :type Vector :default "0, 0, 0") (Hit :type Hit%20Result%20Structure%20%28by%20ref%29))
  ;[1 0.8173 0] Rebondis
  (if (Utilities|Enum|Equal(Enum) (Variables|Default|GetColor) "NewEnumerator2")
    (bind _asbp_first_person (Utilities|Casting|CastToBP_FirstPerson OtherActor))
    (Character|LaunchCharacter _asbp_first_person (Math|Vector|MakeVector 0.0 0.0 (* (Math|Float|Clamp(Float) (.z (Transformation|GetComponentVelocity (Variables|/Script/Engine.Actor|GetRootComponent _asbp_first_person))) -4.2e+03 -4.2e+02) -1.0)) false true)
    (Audio|PlaySoundatLocation "/Game/MyGame/Sound/SoundEffect/SFX_Bounce.SFX_Bounce" (.Location (Collision|BreakHitResult Hit)) "0, 0, 0" 1.0 1.0 0.0 0 0 0 0)))

(event OnComponentBeginOverlap(Box_Haut)
  (params (OverlappedComponent :type Primitive%20Component%20Object%20Reference) (OtherActor :type Actor%20Object%20Reference) (OtherComp :type Primitive%20Component%20Object%20Reference) (OtherBodyIndex :type Integer) (bFromSweep :type Boolean) (SweepResult :type Hit%20Result%20Structure%20%28by%20ref%29))
  ;[1 1 1] Entré et sortie du tapis
  (bind _asgi_main (Utilities|Casting|CastToGI_Main (Game|GetGameInstance)))
  (if (Actor|ActorHasTag OtherActor (Variables|/Game/MyGame/Data/GameInstance/GI_Main.GI_Main_C|GetTagNameTapisRoulant _asgi_main))
    (Utilities|Array|AddUnique (Variables|Default|GetActorOverlaping) OtherActor)
    ;[0.5417 0.1752 0] fin / entré tapis
    (bind _asbp_paintable_cube (Utilities|Casting|CastToBP_PaintableCube OtherActor))))

(event OnComponentEndOverlap(Box_Haut)
  (params (OverlappedComponent :type Primitive%20Component%20Object%20Reference) (OtherActor :type Actor%20Object%20Reference) (OtherComp :type Primitive%20Component%20Object%20Reference) (OtherBodyIndex :type Integer))
  ;[1 1 1] Entré et sortie du tapis
  (bind _asgi_main (Utilities|Casting|CastToGI_Main (Game|GetGameInstance)))
  (if (Actor|ActorHasTag OtherActor (Variables|/Game/MyGame/Data/GameInstance/GI_Main.GI_Main_C|GetTagNameTapisRoulant _asgi_main))
    (Utilities|Array|RemoveItem (Variables|Default|GetActorOverlaping) OtherActor)
    (if (Variables|Default|GetCanPropulse)
      (CallFunction|PROPULSECUBE OtherActor 1.0)
      (else
        ;[0.5417 0.1752 0] fin / entré tapis
        (bind _asbp_paintable_cube (Utilities|Casting|CastToBP_PaintableCube OtherActor)
          (:CastFailed
            (CallFunction|PropulsePasJoueur OtherActor)))))))

(event OnComponentBeginOverlap(Box_Bas)
  (params (OverlappedComponent :type Primitive%20Component%20Object%20Reference) (OtherActor :type Actor%20Object%20Reference) (OtherComp :type Primitive%20Component%20Object%20Reference) (OtherBodyIndex :type Integer) (bFromSweep :type Boolean) (SweepResult :type Hit%20Result%20Structure%20%28by%20ref%29))
  ;[1 1 1] Entré et sortie du tapis
  (bind _asgi_main (Utilities|Casting|CastToGI_Main (Game|GetGameInstance)))
  (if (Actor|ActorHasTag OtherActor (Variables|/Game/MyGame/Data/GameInstance/GI_Main.GI_Main_C|GetTagNameTapisRoulant _asgi_main))
    (Utilities|Array|AddUnique (Variables|Default|GetActorOverlaping_Dessous) OtherActor)
    ;[0.5417 0.1752 0] fin / entré tapis
    (bind _asbp_paintable_cube (Utilities|Casting|CastToBP_PaintableCube OtherActor))))

(event OnComponentEndOverlap(Box_Bas)
  (params (OverlappedComponent :type Primitive%20Component%20Object%20Reference) (OtherActor :type Actor%20Object%20Reference) (OtherComp :type Primitive%20Component%20Object%20Reference) (OtherBodyIndex :type Integer))
  ;[1 1 1] Entré et sortie du tapis
  (bind _asgi_main (Utilities|Casting|CastToGI_Main (Game|GetGameInstance)))
  (if (Actor|ActorHasTag OtherActor (Variables|/Game/MyGame/Data/GameInstance/GI_Main.GI_Main_C|GetTagNameTapisRoulant _asgi_main))
    (Utilities|Array|RemoveItem (Variables|Default|GetActorOverlaping_Dessous) OtherActor)
    (if (Variables|Default|GetCanPropulse)
      (CallFunction|PROPULSECUBE OtherActor -1.0)
      (else
        ;[0.5417 0.1752 0] fin / entré tapis
        (bind _asbp_paintable_cube (Utilities|Casting|CastToBP_PaintableCube OtherActor)
          (:CastFailed
            (CallFunction|PropulsePasJoueur OtherActor)))))))

(event Custom|PROPULSECUBE
  (params (NewParam :type Actor%20Object%20Reference) (Float :type Float%20%28double-precision%29))
  (bind _asbp_paintable_cube (Utilities|Casting|CastToBP_PaintableCube NewParam))
  (if (Physics|IsSimulatingPhysics (Variables|/Game/MyGame/Mech_Color/Paintable/Cube/BP_PaintableCube.BP_PaintableCube_C|GetStaticMesh _asbp_paintable_cube) "None")
    (if (not (Variables|/Game/MyGame/Mech_Color/Paintable/Cube/BP_PaintableCube.BP_PaintableCube_C|GetbIsPickedUp _asbp_paintable_cube))
      (Physics|AddImpulse (Variables|/Game/MyGame/Mech_Color/Paintable/Cube/BP_PaintableCube.BP_PaintableCube_C|GetStaticMesh _asbp_paintable_cube) (* (* (Transformation|GetActorForwardVector) Float) (Variables|Default|GetNewSpeed) (Math|Float|MakeLiteralFloat 1.1e+02)) "None" true))))

(event Custom|OnChangeCouleur
  ;[1 1 1] Color Change
  (if (== (Variables|Default|GetcurrentTrigger) (Variables|Default|GettriggerCount))
    (switch Utilities|FlowControl|Switch|SwitchonEnumColor (Variables|Default|GetColor)
      (:NewEnumerator0
        (bind _output_get (Variables|Default|SetNewSpeed (* (Variables|Default|GetSpeed) -1.0)))
        (Rendering|Material|SetScalarParameterValueonMaterials (Variables|Default|GetStaticMesh) "Speed" _output_get))
      (:NewEnumerator1
        (bind _output_get_2 (Variables|Default|SetNewSpeed (* (Variables|Default|GetSpeed) (Variables|Default|GetRedPush))))
        (Rendering|Material|SetScalarParameterValueonMaterials (Variables|Default|GetStaticMesh) "Speed" _output_get_2))
      (:NewEnumerator2
        (bind _output_get_3 (Variables|Default|SetNewSpeed (Variables|Default|GetSpeed) :!label _label))
        (Rendering|Material|SetScalarParameterValueonMaterials (Variables|Default|GetStaticMesh) "Speed" _output_get_3))
      (:NewEnumerator4
        (goto _label)))
    (else
      (bind _output_get_4 (Variables|Default|SetNewSpeed 0.0))
      (Rendering|Material|SetScalarParameterValueonMaterials (Variables|Default|GetStaticMesh) "Speed" _output_get_4))))

(event Custom|PropulsePasJoueur
  (params (Actor :type Actor%20Object%20Reference))
  (bind _returnvalue (Game|GetPlayerCharacter 0))
  ;[1 0.298 0] Comment
  (if (== Actor _returnvalue)
    (Utilities|FlowControl|Delay 0.1)
    (Variables|/Script/Engine.MovementComponent|SetVelocity (Variables|/Script/Engine.Character|GetCharacterMovement _returnvalue) "0, 0, 0")))

(event Custom|DeplacementDessous
  (bind _returnvalue (Transformation|GetActorForwardVector))
  (bind _returnvalue_2 (* _returnvalue -1.0))
  (for _array_element (Variables|Default|GetActorOverlaping_Dessous)
    ;[0 1 0.9307] Dessous
    ;;[1 1 1] Déplacement cube
    (bind _asbp_paintable_cube (Utilities|Casting|CastToBP_PaintableCube _array_element)
      (:then
        (Transformation|AddActorWorldOffset _asbp_paintable_cube (* (* _returnvalue_2 (Variables|Default|GetNewSpeed) (* (stale EventTick DeltaSeconds) 85.0)) (Math|Float|MakeLiteralFloat 1.12))))
      (:CastFailed
        ;;[1 1 1] Déplacement joueur
        (bind _asbp_first_person (Utilities|Casting|CastToBP_FirstPerson _array_element))
        (Physics|AddImpulse (Variables|/Script/Engine.Character|GetCharacterMovement _asbp_first_person) (* _returnvalue_2 (Variables|Default|GetNewSpeed) (Math|Float|MakeLiteralFloat 5e+01) (* (stale EventTick DeltaSeconds) 85.0)) true)))))

(event EventBeginPlay)

(event EventTick
  (params (DeltaSeconds :type Float%20%28single-precision%29))
  (bind _returnvalue (* DeltaSeconds 85.0))
  (bind _currenttrigger (Variables|Default|GetcurrentTrigger))
  (bind _triggercount (Variables|Default|GettriggerCount))
  (bind _returnvalue_2 (== _currenttrigger _triggercount))
  (Utilities|FlowControl|Sequence
    (:then_0
      (if _returnvalue_2
        (Utilities|FlowControl|Sequence
          (:then_0
            (for _array_element (Variables|Default|GetActorOverlaping)
              ;[1 0 0.05081] Dessus
              ;;[1 1 1] Déplacement cube
              (bind _asbp_paintable_cube (Utilities|Casting|CastToBP_PaintableCube _array_element)
                (:then
                  (Transformation|AddActorWorldOffset _asbp_paintable_cube (* (* (Transformation|GetActorForwardVector) (Variables|Default|GetNewSpeed) _returnvalue) (Math|Float|MakeLiteralFloat 1.12))))
                (:CastFailed
                  ;;[1 1 1] Déplacement joueur
                  (bind _asbp_first_person (Utilities|Casting|CastToBP_FirstPerson _array_element))
                  (Physics|AddImpulse (Variables|/Script/Engine.Character|GetCharacterMovement _asbp_first_person) (* (Transformation|GetActorForwardVector) (Variables|Default|GetNewSpeed) (Math|Float|MakeLiteralFloat 5e+01) _returnvalue) true)))))
          (:then_1
            ;[0 0.9162 1] Call dessous
            (CallFunction|DeplacementDessous)))))
    (:then_1
      (Audio|Components|Audio|SetVolumeMultiplier (Variables|Default|GetSFX) (Math|Float|SelectFloat 1.0 0.0 _returnvalue_2) :!class /Script/Engine.AudioComponent))))

(event EventAction
  (params (currentTrigger :type Integer))
  (CallFunction|OnChangeCouleur))

(event EventChangeColor
  (params (newColor :type EnumColor%20Enum :default "NewEnumerator0"))
  (CallFunction|UpdateMaterial newColor)
  (Audio|PlaySoundatLocation (Utilities|Select :Index (Variables|Default|GetColor) :NewEnumerator0 "/Game/MyGame/Sound/SoundEffect/SFX_PaintableBlue.SFX_PaintableBlue" :NewEnumerator1 "/Game/MyGame/Sound/SoundEffect/SFX_PaintableRed.SFX_PaintableRed" :NewEnumerator2 "/Game/MyGame/Sound/SoundEffect/SFX_PaintableYellow.SFX_PaintableYellow" :NewEnumerator4 "/Game/MyGame/Sound/SoundEffect/SFX_PaintableWhite.SFX_PaintableWhite") (Transformation|GetActorLocation) "0, 0, 0" 1.0 1.0 0.0 0 0 0 0)
  (Audio|Components|Audio|SetSound (Variables|Default|GetSFX) (Utilities|Select :Index (Variables|Default|GetColor) :NewEnumerator0 "/Game/MyGame/Sound/SoundEffect/SFX_TapisLent.SFX_TapisLent" :NewEnumerator1 "/Game/MyGame/Sound/SoundEffect/SFX_TapisRapide.SFX_TapisRapide" :NewEnumerator2 "/Game/MyGame/Sound/SoundEffect/SFX_TapisLent.SFX_TapisLent" :NewEnumerator4 "/Game/MyGame/Sound/SoundEffect/SFX_TapisLent.SFX_TapisLent")))

(fn ConstructionScript
  (bind _returnvalue (Transformation|GetActorUpVector))
  (bind _box_haut (Variables|Default|GetBox_Haut))
  (bind _box_bas (Variables|Default|GetBox_Bas))
  (bind _staticmesh (Variables|Default|GetStaticMesh))
  (bind _tapisscale (Variables|Default|GetTapisScale))
  (bind _returnvalue_2 (Transformation|GetWorldLocation _box_bas))
  (bind _returnvalue_3 (Transformation|GetWorldLocation _box_haut))
  (bind _returnvalue_4 (Transformation|GetWorldLocation _staticmesh))
  (CallFunction|BeginFunction)
  (Utilities|FlowControl|Sequence
    (:then_0
      (Rendering|Material|SetScalarParameterValueonMaterials (Variables|Default|GetStaticMesh) "Speed" (Variables|Default|GetSpeed)))
    (:then_1
      (CallFunction|UpdateMaterial (Variables|Default|GetColor)))
    (:then_2
      (Transformation|SetWorldScale3D (Variables|Default|GetStaticMesh) (Variables|Default|GetTapisScale))
      (Transformation|SetWorldScale3D (Variables|Default|GetBox_Haut) (Math|Vector|MakeVector (.x _tapisscale) (.y _tapisscale) (/ (.z _tapisscale) 2.0)))
      ;[1 1 1] Pour repositionner les box en fonction du tapis roulant
      (Transformation|SetWorldLocation _box_haut (Math|Vector|MakeVector (.x _returnvalue_3) (.y _returnvalue_3) (+ (* (.z (Variables|Default|GetTapisScale)) 2e+02 (.z _returnvalue)) (.z _returnvalue_4))) false false)
      (Transformation|SetWorldLocation _box_bas (Math|Vector|MakeVector (.x _returnvalue_2) (.y _returnvalue_2) (+ (* (.z (Variables|Default|GetTapisScale)) -1e+02 (.z _returnvalue)) (.z _returnvalue_4))) false false)
      (if true
        _))))

(fn UpdateMaterial
  (params (Couleur :type EnumColor%20Enum :default "NewEnumerator0"))
  (bind _colortextures (Variables|Default|GetColorTextures))
  (bind (_mat_none _mat_blue _mat_yellow _mat_red) (Utilities|Struct|BreakStructColorText _colortextures))
  (Variables|Default|SetColor Couleur)
  (for (_array_element _array_index) (Utilities|Select :Index (Variables|Default|GetColor) :NewEnumerator0 _mat_blue :NewEnumerator1 _mat_red :NewEnumerator2 _mat_yellow :NewEnumerator4 _mat_none)
    (Rendering|Material|SetMaterial (Variables|Default|GetStaticMesh) _array_index _array_element)
    (CallFunction|OnChangeCouleur)))

(fn SetFiredonEvent)