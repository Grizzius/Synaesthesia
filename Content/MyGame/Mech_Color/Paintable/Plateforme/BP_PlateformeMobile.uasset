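; Paintable mobile platform whose color sets its behavior: Red moves, Blue can rotate 90 degrees, and Yellow bounces characters along its arrow.
; Color changes swap the material, play a sound and re-evaluate movement through CheckEnergy, which gates on a trigger count.
; A timeline lerps the mesh between offset endpoints with optional ping-pong, its speed set by CustomTimeDilation.
; An attached child actor follows the mesh every tick.
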(event OnComponentHit(PlateformeMesh)
  (params (HitComponent :type Primitive%20Component%20Object%20Reference) (OtherActor :type Actor%20Object%20Reference) (OtherComp :type Primitive%20Component%20Object%20Reference) (NormalImpulse :type Vector :default "0, 0, 0") (Hit :type Hit%20Result%20Structure%20%28by%20ref%29))
  (if (Utilities|Enum|Equal(Enum) (Variables|Default|GetEnumColor) "NewEnumerator2")
    (bind _ascharacter (Utilities|Casting|CastToCharacter OtherActor))
    (Character|LaunchCharacter _ascharacter (* (Math|Vector|VectorLength (Transformation|GetComponentVelocity (Variables|/Script/Engine.Actor|GetRootComponent _ascharacter))) (Math|Vector|Normalize (Math|Vector|GetForwardVector (Variables|Default|GetArrow1))) 0.95) false true)
    (Audio|PlaySoundatLocation "/Game/MyGame/Sound/SoundEffect/SFX_Bounce.SFX_Bounce" (.Location (Collision|BreakHitResult Hit)) "0, 0, 0" 1.0 1.0 0.0 0 0 0 0)))

(event OnComponentEndOverlap(BumpStart)
  (params (OverlappedComponent :type Primitive%20Component%20Object%20Reference) (OtherActor :type Actor%20Object%20Reference) (OtherComp :type Primitive%20Component%20Object%20Reference) (OtherBodyIndex :type Integer))
  (bind _asbp_turret_bullet (Utilities|Casting|CastToBP_TurretBullet OtherActor))
  (Variables|/Game/MyGame/Mech_Color/Paintable/Tourelle/BP_TurretBullet.BP_TurretBullet_C|SetTouchBumpActor _asbp_turret_bullet false))

(event OnComponentBeginOverlap(BumpStart)
  (params (OverlappedComponent :type Primitive%20Component%20Object%20Reference) (OtherActor :type Actor%20Object%20Reference) (OtherComp :type Primitive%20Component%20Object%20Reference) (OtherBodyIndex :type Integer) (bFromSweep :type Boolean) (SweepResult :type Hit%20Result%20Structure%20%28by%20ref%29))
  (if (Utilities|Enum|Equal(Enum) (Variables|Default|GetEnumColor) "NewEnumerator2")
    (bind _asbp_turret_bullet (Utilities|Casting|CastToBP_TurretBullet OtherActor))
    (Variables|/Game/MyGame/Mech_Color/Paintable/Tourelle/BP_TurretBullet.BP_TurretBullet_C|SetTouchBumpActor _asbp_turret_bullet true)))

(event Custom|EventStopPlatform
  (bind _movingsound (Variables|Default|GetMovingSound))
  (if (not (Variables|Default|GetForMehdi))
    (Audio|Components|Audio|SetVolumeMultiplier _movingsound 0.0 :!class /Script/Engine.AudioComponent)
    (bind (_direction _newtrack_0) (Timeline|Timeline_0 Stop)
      (:Update
        (Audio|Components|Audio|SetVolumeMultiplier (Variables|Default|GetMovingSound) 1.0 :!class /Script/Engine.AudioComponent)
        (Transformation|SetWorldLocation (Variables|Default|GetPlateformeMesh) (Math|Vector|Lerp(Vector) (Variables|Default|GetBeginLoc) (Variables|Default|GetEndLoc) _newtrack_0) false false))
      (:Finished
        (Audio|Components|Audio|SetVolumeMultiplier _movingsound 0.0 :!class /Script/Engine.AudioComponent)
        (switch Utilities|FlowControl|Switch|SwitchonETimelineDirection _direction
          (:Forward
            (if (Variables|Default|GetbPingPong)
              (Timeline|Timeline_0 Reverse)))
          (:Backward
            (Utilities|CheckEnergy
              (:enoughEnergy
                (Timeline|Timeline_0 Play)))))))
    (else
      (Timeline|Timeline_0 Reverse))))

(event Custom|EventStartPlatform
  (if (Utilities|Enum|Equal(Enum) (Variables|Default|GetEnumColor) "NewEnumerator1")
    (switch Utilities|FlowControl|Switch|SwitchonETimelineDirection (stale _direction)
      (:Forward
        (bind (_direction _newtrack_0) (Timeline|Timeline_0 Play)
          (:Update
            (Audio|Components|Audio|SetVolumeMultiplier (Variables|Default|GetMovingSound) 1.0 :!class /Script/Engine.AudioComponent)
            (Transformation|SetWorldLocation (Variables|Default|GetPlateformeMesh) (Math|Vector|Lerp(Vector) (Variables|Default|GetBeginLoc) (Variables|Default|GetEndLoc) _newtrack_0) false false))
          (:Finished
            (Audio|Components|Audio|SetVolumeMultiplier (Variables|Default|GetMovingSound) 0.0 :!class /Script/Engine.AudioComponent)
            (switch Utilities|FlowControl|Switch|SwitchonETimelineDirection _direction
              (:Forward
                (if (Variables|Default|GetbPingPong)
                  (Timeline|Timeline_0 Reverse)))
              (:Backward
                (Utilities|CheckEnergy
                  (:enoughEnergy
                    (Timeline|Timeline_0 Play))))))))
      (:Backward
        (Timeline|Timeline_0 Reverse)))))

(event Custom|EventOnChangeColor
  (bind _plateformemesh (Variables|Default|GetPlateformeMesh))
  (bind _defaultrotation (Variables|Default|GetDefaultRotation))
  (bind _defaultrotation_2 (Variables|Default|GetDefaultRotation))
  (bind _defaultrotation_3 (Variables|Default|GetDefaultRotation))
  (bind _defaultrotation_4 (Variables|Default|GetDefaultRotation))
  (bind (_roll _pitch _yaw) (Math|Rotator|BreakRotator _defaultrotation))
  (bind (_roll_2 _pitch_2 _yaw_2) (Math|Rotator|BreakRotator _defaultrotation_2))
  (bind (_roll_3 _pitch_3 _yaw_3) (Math|Rotator|BreakRotator _defaultrotation_3))
  (bind (_roll_4 _pitch_4 _yaw_4) (Math|Rotator|BreakRotator _defaultrotation_4))
  (Utilities|CheckEnergy
    (:enoughEnergy
      (Default|CallStartPlatform))
    (:notEnoughEnergy
      (CallFunction|EventStopPlatform)))
  (Variables|Default|SetCustomTimeDilation (Variables|Default|Getspeed))
  (Transformation|SetRelativeRotation (Variables|Default|GetPlateformeMesh) (Variables|Default|GetDefaultRotation) false false)
  (switch Utilities|FlowControl|Switch|SwitchonEnumColor (Variables|Default|GetEnumColor)
    (:NewEnumerator0
      (Utilities|FlowControl|Sequence
        (:then_0
          (if (Variables|Default|GetRota%2090y)
            (Transformation|SetRelativeRotation _plateformemesh (Math|Rotator|MakeRotator _roll_2 (+ _pitch_2 9e+01) _yaw_2) false false)
            (elif (Variables|Default|GetRota%20-90x)
              (Transformation|SetRelativeRotation _plateformemesh (Math|Rotator|MakeRotator (+ _roll_3 9e+01) _pitch_3 _yaw_3) false false)
              (elif (Variables|Default|GetRota%20-90y)
                (Transformation|SetRelativeRotation _plateformemesh (Math|Rotator|MakeRotator _roll_4 (+ _pitch_4 -9e+01) _yaw_4) false false)
                (elif (Variables|Default|GetRota%2090x)
                  (Transformation|SetRelativeRotation _plateformemesh (Math|Rotator|MakeRotator (+ _roll 9e+01) _pitch _yaw) false false))))))
        (:then_1
          (CallFunction|EventStopPlatform :!label _label))))
    (:NewEnumerator2
      (goto _label))
    (:NewEnumerator4
      (goto _label))))

(event EventBeginPlay
  (Utilities|FlowControl|Sequence
    (:then_0
      (CallFunction|SetFiredonEvent))
    (:then_1
      (Variables|Default|SetCustomTimeDilation (Variables|Default|Getspeed))
      (CallFunction|BeginFunction)
      (Variables|Default|SetBeginLoc (+ (Transformation|GetActorLocation) (Variables|Default|GetBeginLoc)))
      (Variables|Default|SetEndLoc (+ (Variables|Default|GetEndLoc) (Transformation|GetActorLocation)))
      (Components|Timeline|SetNewTime (Variables|Default|GetTimeline_0) (Variables|Default|GetNewtime))
      (EventDispatchers|BindEventtoNewEventDispatcher0 (delegate Custom|EventOnChangeColor))
      (EventDispatchers|BindEventtoStartPlatform (delegate Custom|EventStartPlatform))
      (Utilities|CheckEnergy
        (:enoughEnergy
          (CallFunction|EventStartPlatform)
          (CallFunction|EventonChangeColor))))
    (:then_2
      (Variables|Default|SetDefaultRotation (Variables|/Script/Engine.SceneComponent|GetRelativeRotation (Variables|Default|GetPlateformeMesh))))))

(event EventChangeColor
  (params (newColor :type EnumColor%20Enum :default "NewEnumerator0"))
  (CallFunction|UpdateMaterial newColor)
  (Audio|PlaySoundatLocation (Utilities|Select :Index (Variables|Default|GetEnumColor) :NewEnumerator0 "/Game/MyGame/Sound/SoundEffect/SFX_PaintableBlue.SFX_PaintableBlue" :NewEnumerator1 "/Game/MyGame/Sound/SoundEffect/SFX_PaintableRed.SFX_PaintableRed" :NewEnumerator2 "/Game/MyGame/Sound/SoundEffect/SFX_PaintableYellow.SFX_PaintableYellow" :NewEnumerator4 "/Game/MyGame/Sound/SoundEffect/SFX_PaintableWhite.SFX_PaintableWhite") (Transformation|GetActorLocation) "0, 0, 0" 1.0 1.0 0.0 0 0 0 0))

(event EventTick
  (params (DeltaSeconds :type Float%20%28single-precision%29))
  (CallFunction|SetChildActorPosition))

(event EventAction
  (params (currentTrigger :type Integer))
  (Utilities|CheckEnergy
    (:enoughEnergy
      (if (not (Variables|Default|GetForMehdi))
        (CallFunction|EventStartPlatform)
        (else
          (CallFunction|EventStopPlatform :!label _label))))
    (:notEnoughEnergy
      (goto _label))))

(fn ConstructionScript
  (CallFunction|ConstructionFunction)
  (Rendering|Material|SetMaterial (Variables|Default|GetPlateformeMesh) 0 (Utilities|Array|Get(acopy) (Variables|Default|GetColorMaterials) (Utilities|Select :Index (Variables|Default|GetEnumColor) :NewEnumerator0 2 :NewEnumerator1 1 :NewEnumerator2 3 :NewEnumerator4 0)))
  (Transformation|SetWorldScale3D (Variables|Default|GetArrow1) "1.000000,1.000000,1.000000")
  (CallFunction|SetChildActorPosition)
  (Components|StaticMesh|SetStaticMesh (Variables|Default|GetPlateformeMesh) (select (Variables|Default|GetbIsCut) "/Game/MyGame/3D_Assets/platform/platform_cut.platform_cut" "/Game/MyGame/3D_Assets/platform/SM_MERGED_StaticMeshActor_1179.SM_MERGED_StaticMeshActor_1179")))

(fn UpdateMaterial
  (params (newColor :type EnumColor%20Enum :default "NewEnumerator0"))
  (Variables|Default|SetEnumColor newColor)
  (Rendering|Material|SetMaterial (Variables|Default|GetPlateformeMesh) 0 (Utilities|Array|Get(acopy) (Variables|Default|GetColorMaterials) (Utilities|Select :Index (Variables|Default|GetEnumColor) :NewEnumerator0 2 :NewEnumerator1 1 :NewEnumerator2 3 :NewEnumerator4 0)))
  (Default|CallNewEventDispatcher0))

(fn ResetColor)

(fn SetChildActorPosition
  (bind _childactorpivot (Variables|Default|GetChildActorPivot))
  (bind _childactor (Variables|ChildActor|GetchildActor))
  (bind _childactorrotation (Variables|ChildActor|GetchildActorRotation))
  (Utilities|IsValid _childactor
    (:Is%20Valid
      (bind _asbp_color_detector (Utilities|Casting|CastToBP_ColorDetector _childactor)
        (:then
          (Variables|/Game/MyGame/Mech_Env/ColorDetector/BP_ColorDetector.BP_ColorDetector_C|SetparentPlatform _asbp_color_detector self))
        (:CastFailed
          _))
      (Transformation|SetActorLocation (Variables|ChildActor|GetchildActor) (+ (Transformation|GetWorldLocation (Variables|Default|GetPlateformeMesh)) (Variables|ChildActor|GetchildActorOffset)) false false)
      (Transformation|SetRelativeRotation _childactorpivot (Math|Rotator|MakeRotator (.x _childactorrotation) (.y _childactorrotation) (.z _childactorrotation)) false false)
      (Transformation|SetActorRotation (Variables|ChildActor|GetchildActor) (Transformation|GetWorldRotation _childactorpivot)))))

(fn SetFiredonEvent)

(fn ReturnBounceAngle
  (params (Vector%20A :type Vector) (Vector%20B :type Vector))
  (return (Class|KismetMathLibrary|DegAcos (Math|Vector|DotProduct (Math|Vector|Normalize Vector%20A) (Math|Vector|Normalize Vector%20B)))))