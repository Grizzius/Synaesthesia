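; Activable door Blueprint that opens when the trigger count passed to its Action event equals TriggerCount.
; BeginPlay caches the start location and calls BeginFunction.
; Opening instantly sets the relative location far up on Z and plays the open sound, while any other count restores the cached location.
; A DoOnce, reset on each opening, keeps the close sound from repeating until the door opens again.
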(event EventBeginPlay
  (Variables|Default|SetLocationStart (Transformation|GetActorLocation))
  (CallFunction|BeginFunction))

(event EventAction
  (params (currentTrigger :type Integer))
  (if (== currentTrigger (Variables|Default|GettriggerCount))
    (Transformation|SetActorRelativeLocation "0.000000,0.000000,10000.000000")
    (Audio|PlaySoundatLocation "/Game/MyGame/Sound/SoundEffect/SFX_DoorOpen.SFX_DoorOpen" (Transformation|GetActorLocation) "0, 0, 0" 1.0 1.0 0.0 0 0 0 0)
    (goto _label Reset)
    (else
      (Transformation|SetActorRelativeLocation (Variables|Default|GetLocationStart))
      (Utilities|FlowControl|DoOnce false :!label _label
        (:Completed
          (Audio|PlaySoundatLocation "/Game/MyGame/Sound/SoundEffect/SFX_DoorClose.SFX_DoorClose" (Transformation|GetActorLocation) "0, 0, 0" 1.0 1.0 0.0 0 0 0 0))))))

(fn ConstructionScript)