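; Bp_Lightdoor is an environment mechanism whose sphere acts as a status light for a set of triggers.
; Its Action event turns the sphere green when CurrentTrigger equals the TriggerSet length, and violet otherwise.
; BeginPlay runs BeginFunction and then Action to set the starting color, while the construction script delegates to ConstructionFunction.
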(event Collision|EventActorBeginOverlap
  (params (OtherActor :type Actor%20Object%20Reference)))

(event EventAction
  (params (currentTrigger :type Integer))
  (Rendering|Material|SetMaterial (Variables|Default|GetSphere) 0 (select (== currentTrigger (Utilities|Set|Length (Variables|Default|GetTriggerSet))) "/Game/MyGame/Materials/MI_LedGreen.MI_LedGreen" "/Game/MyGame/Materials/MI_LedViolet_2.MI_LedViolet_2")))

(event EventBeginPlay
  (CallFunction|BeginFunction)
  (CallFunction|Action (Variables|Default|GetcurrentTrigger)))

(fn ConstructionScript
  (CallFunction|ConstructionFunction))