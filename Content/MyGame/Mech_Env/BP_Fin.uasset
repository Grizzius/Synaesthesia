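; BP_Fin is the interactable end-of-game actor that calls GameEnd on GM_InGame when the player interacts with it.
; On BeginPlay it reads ProgressionState from GI_Main and destroys itself in the listed earlier states, from Begin Game through Completed Level 2.
; Interact HUD events show and hide its prompt Widget.
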(event EventBeginPlay
  (bind _asgi_main (Utilities|Casting|CastToGI_Main (Game|GetGameInstance)))
  (switch Utilities|FlowControl|Switch|SwitchonProgressionState (Variables|/Game/MyGame/Data/GameInstance/GI_Main.GI_Main_C|GetProgressionState _asgi_main)
    (:NewEnumerator0
      _)
    (:NewEnumerator6
      _)
    (:NewEnumerator1
      _)
    (:NewEnumerator2
      _))
  (Actor|DestroyActor))

(event Collision|EventActorBeginOverlap
  (params (OtherActor :type Actor%20Object%20Reference)))

(event EventTick
  (params (DeltaSeconds :type Float%20%28single-precision%29)))

(event EventOnInteract
  (params (Player%20Ref :type BP%20First%20Person%20Object%20Reference))
  (bind _asgm_in_game (Utilities|Casting|CastToGM_InGame (Game|GetGameMode)))
  (Default|GameEnd _asgm_in_game))

(event EventDisplayInteractHUD
  (Rendering|SetVisibility (Variables|Default|GetWidget) true false))

(event EventHideInteractHUD
  (Rendering|SetVisibility (Variables|Default|GetWidget) false false))

(fn ConstructionScript)