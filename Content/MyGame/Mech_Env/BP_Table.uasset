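; BP_Table is an environment table whose displayed props depend on the game's progression.
; On BeginPlay it reads ProgressionState from GI_Main and destroys the components that should not yet show.
; Early states remove the typewriter, helmet and both piles; completing Level 1 keeps the helmet, and Level 2 also keeps the typewriter.
; States without a wired branch leave every prop in place.
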(event EventBeginPlay
  (bind _asgi_main (Utilities|Casting|CastToGI_Main (Game|GetGameInstance)))
  (switch Utilities|FlowControl|Switch|SwitchonProgressionState (Variables|/Game/MyGame/Data/GameInstance/GI_Main.GI_Main_C|GetProgressionState _asgi_main)
    (:NewEnumerator0
      (Components|DestroyComponent (Variables|Default|Getmachine_ecrire) :!label _label))
    (:NewEnumerator6
      (goto _label))
    (:NewEnumerator1
      (Components|DestroyComponent (Variables|Default|GetPile_2)))
    (:NewEnumerator2
      (Components|DestroyComponent (Variables|Default|GetPile_1)))))

(event Collision|EventActorBeginOverlap
  (params (OtherActor :type Actor%20Object%20Reference)))

(event EventTick
  (params (DeltaSeconds :type Float%20%28single-precision%29)))

(fn ConstructionScript)