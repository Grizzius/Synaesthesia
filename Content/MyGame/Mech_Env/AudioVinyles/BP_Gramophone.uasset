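; BP_Gramophone is an interactable gramophone that plays narrated vinyl records with subtitles.
; Interacting pauses the game, shows the cursor and opens WB_Gramophone with a self reference, while HUD events toggle the interact prompt widget.
; PlayVinyle steps through a vinyl's audio entries in a Delay-driven loop, playing each as 2D sound and updating a WB_Subtitle created at BeginPlay, removed after the last entry.
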(event Custom|PlayVinyle
  (params (Vinyle :type Struct%20Vinyle%20Structure))
  (bind _audio (Utilities|Struct|BreakStruct_Vinyle Vinyle))
  (bind _subtitlewidget (Variables|Default|GetSubtitleWidget))
  (Variables|Default|SetVinyleAudioID 0)
  (if (< (Variables|Default|GetVinyleAudioID) (Utilities|Array|Length _audio)) :!label _label
    (Audio|PlaySound2D (.audio (Utilities|Struct|BreakStruct_VinyleAudio (Utilities|Array|Get(acopy) _audio (Variables|Default|GetVinyleAudioID)))) 1.0 1.0 0.0 0 0)
    (UserInterface|Viewport|AddtoViewport _subtitlewidget 0)
    (Variables|/Game/MyGame/Mech_Env/AudioVinyles/WB_Subtitle.WB_Subtitle_C|SetText _subtitlewidget (.Text (Utilities|Struct|BreakStruct_VinyleAudio (Utilities|Array|Get(acopy) _audio (Variables|Default|GetVinyleAudioID)))))
    (Utilities|FlowControl|Delay (.Durée (Utilities|Struct|BreakStruct_VinyleAudio (Utilities|Array|Get(acopy) _audio (Variables|Default|GetVinyleAudioID)))))
    (Math|Integer|IncrementInt (Variables|Default|GetVinyleAudioID)
      (:%20%20
        (goto _label)))
    (else
      (Widget|RemovefromParent (Variables|Default|GetSubtitleWidget)))))

(event EventBeginPlay
  (bind _returnvalue (UserInterface|CreateWidget "/Game/MyGame/Mech_Env/AudioVinyles/WB_Subtitle.WB_Subtitle_C"))
  (Variables|Default|SetSubtitleWidget _returnvalue))

(event Collision|EventActorBeginOverlap
  (params (OtherActor :type Actor%20Object%20Reference)))

(event EventTick
  (params (DeltaSeconds :type Float%20%28single-precision%29)))

(event EventOnInteract
  (params (Player%20Ref :type BP%20First%20Person%20Object%20Reference))
  (Game|SetGamePaused true)
  (Variables|/Script/Engine.PlayerController|SetbShowMouseCursor (Game|GetPlayerController 0) true)
  (bind _returnvalue (UserInterface|CreateWidget "/Game/MyGame/Mech_Env/AudioVinyles/WB_Gramophone.WB_Gramophone_C" 0 self))
  (UserInterface|Viewport|AddtoViewport _returnvalue 0))

(event EventDisplayInteractHUD
  (Rendering|SetVisibility (Variables|Default|GetWidget) true false))

(event EventHideInteractHUD
  (Rendering|SetVisibility (Variables|Default|GetWidget) false false))

(fn ConstructionScript)