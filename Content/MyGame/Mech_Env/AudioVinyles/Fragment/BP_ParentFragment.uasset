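; Parent Blueprint for collectible fragments that trigger dialogue when they receive their activation color.
; On the first matching ChangeColor, it sets the fragment's numbered flag in GI_Main's StructFragment and hands itself and its dialogue to GM_InGame.
; It estimates dialogue length from each line's character count with a per-line minimum, then destroys its skeletal and Niagara actors and itself after that delay.
; An unconnected level-sequence playback path never runs.
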(event EventBeginPlay
  (Components|Animation|SetAnimation (Variables|Character|GetMesh) "/Game/MyGame/Mech_Env/AudioVinyles/Fragment/FBX/Soldat/Rifle_Aiming_Idle_Anim_mixamo_com.Rifle_Aiming_Idle_Anim_mixamo_com"))

(event Collision|EventActorBeginOverlap
  (params (OtherActor :type Actor%20Object%20Reference)))

(event EventTick
  (params (DeltaSeconds :type Float%20%28single-precision%29)))

(event EventChangeColor
  (params (newColor :type EnumColor%20Enum :default "NewEnumerator0"))
  (bind _dureedialogueminimum (Variables|Default|GetDureeDialogueMinimum))
  (if (Utilities|Enum|Equal(Enum) newColor (Variables|Default|GetColorToActive))
    (if (not (Variables|Default|GetDoOne))
      (Variables|Default|SetDoOne true)
      (bind _asgi_main (Utilities|Casting|CastToGI_Main (Game|GetGameInstance)))
      (switch int (Variables|Default|GetNumero%20du%20fragment)
        (:1
          (Variables|/Game/MyGame/Data/GameInstance/GI_Main.GI_Main_C|SetStruct_fragment _asgi_main (Utilities|Struct|MakeStruct_activate_fragment true (.fargment2 (Variables|/Game/MyGame/Data/GameInstance/GI_Main.GI_Main_C|GetStruct_fragment _asgi_main)) (.fargment3 (Variables|/Game/MyGame/Data/GameInstance/GI_Main.GI_Main_C|GetStruct_fragment _asgi_main)) (.fargment4 (Variables|/Game/MyGame/Data/GameInstance/GI_Main.GI_Main_C|GetStruct_fragment _asgi_main)) (.fargment5 (Variables|/Game/MyGame/Data/GameInstance/GI_Main.GI_Main_C|GetStruct_fragment _asgi_main)) (.fargment6 (Variables|/Game/MyGame/Data/GameInstance/GI_Main.GI_Main_C|GetStruct_fragment _asgi_main)) (.fargment7 (Variables|/Game/MyGame/Data/GameInstance/GI_Main.GI_Main_C|GetStruct_fragment _asgi_main)) (.fargment8 (Variables|/Game/MyGame/Data/GameInstance/GI_Main.GI_Main_C|GetStruct_fragment _asgi_main)))))
        (:2
          (Variables|/Game/MyGame/Data/GameInstance/GI_Main.GI_Main_C|SetStruct_fragment _asgi_main (Utilities|Struct|MakeStruct_activate_fragment (.fargment1 (Variables|/Game/MyGame/Data/GameInstance/GI_Main.GI_Main_C|GetStruct_fragment _asgi_main)) true (.fargment3 (Variables|/Game/MyGame/Data/GameInstance/GI_Main.GI_Main_C|GetStruct_fragment _asgi_main)) (.fargment4 (Variables|/Game/MyGame/Data/GameInstance/GI_Main.GI_Main_C|GetStruct_fragment _asgi_main)) (.fargment5 (Variables|/Game/MyGame/Data/GameInstance/GI_Main.GI_Main_C|GetStruct_fragment _asgi_main)) (.fargment6 (Variables|/Game/MyGame/Data/GameInstance/GI_Main.GI_Main_C|GetStruct_fragment _asgi_main)) (.fargment7 (Variables|/Game/MyGame/Data/GameInstance/GI_Main.GI_Main_C|GetStruct_fragment _asgi_main)) (.fargment8 (Variables|/Game/MyGame/Data/GameInstance/GI_Main.GI_Main_C|GetStruct_fragment _asgi_main)))))
        (:3
          (Variables|/Game/MyGame/Data/GameInstance/GI_Main.GI_Main_C|SetStruct_fragment _asgi_main (Utilities|Struct|MakeStruct_activate_fragment (.fargment1 (Variables|/Game/MyGame/Data/GameInstance/GI_Main.GI_Main_C|GetStruct_fragment _asgi_main)) (.fargment2 (Variables|/Game/MyGame/Data/GameInstance/GI_Main.GI_Main_C|GetStruct_fragment _asgi_main)) true (.fargment4 (Variables|/Game/MyGame/Data/GameInstance/GI_Main.GI_Main_C|GetStruct_fragment _asgi_main)) (.fargment5 (Variables|/Game/MyGame/Data/GameInstance/GI_Main.GI_Main_C|GetStruct_fragment _asgi_main)) (.fargment6 (Variables|/Game/MyGame/Data/GameInstance/GI_Main.GI_Main_C|GetStruct_fragment _asgi_main)) (.fargment7 (Variables|/Game/MyGame/Data/GameInstance/GI_Main.GI_Main_C|GetStruct_fragment _asgi_main)) (.fargment8 (Variables|/Game/MyGame/Data/GameInstance/GI_Main.GI_Main_C|GetStruct_fragment _asgi_main)))))
        (:4
          (Variables|/Game/MyGame/Data/GameInstance/GI_Main.GI_Main_C|SetStruct_fragment _asgi_main (Utilities|Struct|MakeStruct_activate_fragment (.fargment1 (Variables|/Game/MyGame/Data/GameInstance/GI_Main.GI_Main_C|GetStruct_fragment _asgi_main)) (.fargment2 (Variables|/Game/MyGame/Data/GameInstance/GI_Main.GI_Main_C|GetStruct_fragment _asgi_main)) (.fargment3 (Variables|/Game/MyGame/Data/GameInstance/GI_Main.GI_Main_C|GetStruct_fragment _asgi_main)) true (.fargment5 (Variables|/Game/MyGame/Data/GameInstance/GI_Main.GI_Main_C|GetStruct_fragment _asgi_main)) (.fargment6 (Variables|/Game/MyGame/Data/GameInstance/GI_Main.GI_Main_C|GetStruct_fragment _asgi_main)) (.fargment7 (Variables|/Game/MyGame/Data/GameInstance/GI_Main.GI_Main_C|GetStruct_fragment _asgi_main)) (.fargment8 (Variables|/Game/MyGame/Data/GameInstance/GI_Main.GI_Main_C|GetStruct_fragment _asgi_main)))))
        (:5
          (Variables|/Game/MyGame/Data/GameInstance/GI_Main.GI_Main_C|SetStruct_fragment _asgi_main (Utilities|Struct|MakeStruct_activate_fragment (.fargment1 (Variables|/Game/MyGame/Data/GameInstance/GI_Main.GI_Main_C|GetStruct_fragment _asgi_main)) (.fargment2 (Variables|/Game/MyGame/Data/GameInstance/GI_Main.GI_Main_C|GetStruct_fragment _asgi_main)) (.fargment3 (Variables|/Game/MyGame/Data/GameInstance/GI_Main.GI_Main_C|GetStruct_fragment _asgi_main)) (.fargment4 (Variables|/Game/MyGame/Data/GameInstance/GI_Main.GI_Main_C|GetStruct_fragment _asgi_main)) true (.fargment6 (Variables|/Game/MyGame/Data/GameInstance/GI_Main.GI_Main_C|GetStruct_fragment _asgi_main)) (.fargment7 (Variables|/Game/MyGame/Data/GameInstance/GI_Main.GI_Main_C|GetStruct_fragment _asgi_main)) (.fargment8 (Variables|/Game/MyGame/Data/GameInstance/GI_Main.GI_Main_C|GetStruct_fragment _asgi_main)))))
        (:6
          (Variables|/Game/MyGame/Data/GameInstance/GI_Main.GI_Main_C|SetStruct_fragment _asgi_main (Utilities|Struct|MakeStruct_activate_fragment (.fargment1 (Variables|/Game/MyGame/Data/GameInstance/GI_Main.GI_Main_C|GetStruct_fragment _asgi_main)) (.fargment2 (Variables|/Game/MyGame/Data/GameInstance/GI_Main.GI_Main_C|GetStruct_fragment _asgi_main)) (.fargment3 (Variables|/Game/MyGame/Data/GameInstance/GI_Main.GI_Main_C|GetStruct_fragment _asgi_main)) (.fargment4 (Variables|/Game/MyGame/Data/GameInstance/GI_Main.GI_Main_C|GetStruct_fragment _asgi_main)) (.fargment5 (Variables|/Game/MyGame/Data/GameInstance/GI_Main.GI_Main_C|GetStruct_fragment _asgi_main)) true (.fargment7 (Variables|/Game/MyGame/Data/GameInstance/GI_Main.GI_Main_C|GetStruct_fragment _asgi_main)) (.fargment8 (Variables|/Game/MyGame/Data/GameInstance/GI_Main.GI_Main_C|GetStruct_fragment _asgi_main)))))
        (:7
          (Variables|/Game/MyGame/Data/GameInstance/GI_Main.GI_Main_C|SetStruct_fragment _asgi_main (Utilities|Struct|MakeStruct_activate_fragment (.fargment1 (Variables|/Game/MyGame/Data/GameInstance/GI_Main.GI_Main_C|GetStruct_fragment _asgi_main)) (.fargment2 (Variables|/Game/MyGame/Data/GameInstance/GI_Main.GI_Main_C|GetStruct_fragment _asgi_main)) (.fargment3 (Variables|/Game/MyGame/Data/GameInstance/GI_Main.GI_Main_C|GetStruct_fragment _asgi_main)) (.fargment4 (Variables|/Game/MyGame/Data/GameInstance/GI_Main.GI_Main_C|GetStruct_fragment _asgi_main)) (.fargment5 (Variables|/Game/MyGame/Data/GameInstance/GI_Main.GI_Main_C|GetStruct_fragment _asgi_main)) (.fargment6 (Variables|/Game/MyGame/Data/GameInstance/GI_Main.GI_Main_C|GetStruct_fragment _asgi_main)) true (.fargment8 (Variables|/Game/MyGame/Data/GameInstance/GI_Main.GI_Main_C|GetStruct_fragment _asgi_main)))))
        (:8
          (Variables|/Game/MyGame/Data/GameInstance/GI_Main.GI_Main_C|SetStruct_fragment _asgi_main (Utilities|Struct|MakeStruct_activate_fragment (.fargment1 (Variables|/Game/MyGame/Data/GameInstance/GI_Main.GI_Main_C|GetStruct_fragment _asgi_main)) (.fargment2 (Variables|/Game/MyGame/Data/GameInstance/GI_Main.GI_Main_C|GetStruct_fragment _asgi_main)) (.fargment3 (Variables|/Game/MyGame/Data/GameInstance/GI_Main.GI_Main_C|GetStruct_fragment _asgi_main)) (.fargment4 (Variables|/Game/MyGame/Data/GameInstance/GI_Main.GI_Main_C|GetStruct_fragment _asgi_main)) (.fargment5 (Variables|/Game/MyGame/Data/GameInstance/GI_Main.GI_Main_C|GetStruct_fragment _asgi_main)) (.fargment6 (Variables|/Game/MyGame/Data/GameInstance/GI_Main.GI_Main_C|GetStruct_fragment _asgi_main)) (.fargment7 (Variables|/Game/MyGame/Data/GameInstance/GI_Main.GI_Main_C|GetStruct_fragment _asgi_main)) true))))
      ;[0.4375 0.02962 0.06844 0.318] Marouflage pour que le fragment disparaisse a la fin du dialogue
      (for _array_element (Variables|Default|GetDialogue)
        (Variables|Default|SetTotalTimeDialogue (+ (Variables|Default|GetTotalTimeDialogue) (Math|Float|SelectFloat _dureedialogueminimum (* (Variables|Default|GetDureeDialogue) (Utilities|String|Len (Utilities|String|ToString(Text) (.Lignededialogue (Utilities|Struct|BreakS_LigneDeDialogue _array_element))))) (> _dureedialogueminimum (* (Variables|Default|GetDureeDialogue) (Utilities|String|Len (Utilities|String|ToString(Text) (.Lignededialogue (Utilities|Struct|BreakS_LigneDeDialogue _array_element))))))))))
      (bind _asgm_in_game (Utilities|Casting|CastToGM_InGame (Game|GetGameMode)))
      (Variables|/Game/MyGame/Data/GameInstance/GM_InGame.GM_InGame_C|SetCurrentFragment _asgm_in_game self)
      (Default|EventDialogue _asgm_in_game (Variables|Default|GetDialogue))
      (Utilities|FlowControl|Delay (Variables|Default|GetTotalTimeDialogue))
      (Actor|DestroyActor (Variables|Default|GetSkeletal_ref))
      (Actor|DestroyActor (Variables|Default|GetNiagara_ref))
      (Actor|DestroyActor))))

(fn ConstructionScript)