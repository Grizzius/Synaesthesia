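; BP_PorteEnigme is a puzzle door that opens when the trigger count it receives matches its required count.
; The construction script applies the configurable door mesh and transform offset to the static mesh.
; The Action event compares CurrentTrigger with TriggerCount, then snaps the mesh up on a match or back to the relative origin otherwise, with no animation, overriding the offset's location.
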(event EventBeginPlay)

(event Collision|EventActorBeginOverlap
  (params (OtherActor :type Actor%20Object%20Reference)))

(event EventTick
  (params (DeltaSeconds :type Float%20%28single-precision%29)))

(event EventAction
  (params (currentTrigger :type Integer))
  (Transformation|SetRelativeLocation (Variables|Default|GetStaticMesh) (Math|Vector|SelectVector "0.000000,0.000000,200.000000" "0, 0, 0" (== currentTrigger (Variables|Default|GettriggerCount))) false false))

(fn ConstructionScript
  (bind _staticmesh (Variables|Default|GetStaticMesh))
  (Components|StaticMesh|SetStaticMesh _staticmesh (Variables|Default|GetDoorMesh))
  (Transformation|SetRelativeTransform _staticmesh (Variables|Default|GettransformOffset) false false))