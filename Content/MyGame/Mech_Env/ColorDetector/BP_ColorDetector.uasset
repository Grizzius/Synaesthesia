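; Color detector puzzle trigger that activates while a paintable cube or activable conveyor of its color sits visibly in its beam.
; Each tick it filters capsule overlaps by color and sphere-trace line of sight, then fires begin trigger with a sound, or end trigger on every unmatched tick.
; A line trace ignoring paintable cubes resizes the capsule, Niagara beam and spotlight to the first obstruction.
; The construction script tints mesh, beam and light by color.
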(event EventTick
  (params (DeltaSeconds :type Float%20%28single-precision%29))
  (Utilities|FlowControl|Sequence
    (:then_1
      (Variables|Default|SetbFoundColor false)
      (for _array_element (Collision|GetOverlappingActors (Variables|Default|GetCapsule) 0 :!class /Script/Engine.PrimitiveComponent)
        (bind _asbp_paintable_cube (Utilities|Casting|CastToBP_PaintableCube _array_element)
          (:then
            (bind _bobjecthit (CallFunction|CheckObjectinSight _asbp_paintable_cube))
            (if (and _bobjecthit (Utilities|Enum|Equal(Enum) (Variables|/Game/MyGame/Mech_Color/Paintable/Cube/BP_PaintableCube.BP_PaintableCube_C|GetColor _asbp_paintable_cube) (Variables|Default|GetColor)))
              (Variables|Default|SetbFoundColor true :!label _label)
              (if (not (Variables|Default|GetbIsActivated))
                (Variables|Default|SetbIsActivated true)
                (Default|CallBeginTrigger)
                (Audio|PlaySound2D "/Game/MyGame/Sound/SoundEffect/SFX_DetectColor.SFX_DetectColor" 1.0 1.0 0.0 0 0))))
          (:CastFailed
            (bind _asbp_activable_conveyor (Utilities|Casting|CastToBP_ActivableConveyor _array_element))
            (bind _bobjecthit_2 (CallFunction|CheckObjectinSight _asbp_activable_conveyor))
            (if (and _bobjecthit_2 (Utilities|Enum|Equal(Enum) (Variables|/Game/MyGame/Mech_Color/Paintable/Tapis/BP_ActivableConveyor.BP_ActivableConveyor_C|GetColor _asbp_activable_conveyor) (Variables|Default|GetColor)))
              (goto _label)))))
      (if (not (Variables|Default|GetbFoundColor))
        (Variables|Default|SetbIsActivated false)
        (Default|CallEndTrigger)))
    (:then_2
      (CallFunction|CalculateHeight))))

(fn ConstructionScript
  (bind _color (Variables|Default|GetColor))
  (bind _returnvalue (Utilities|Select :Index _color :NewEnumerator0 "(R=0.000000,G=0.000000,B=1.000000,A=1.000000)" :NewEnumerator1 "(R=1.000000,G=0.000000,B=0.000000,A=1.000000)" :NewEnumerator2 "(R=1.000000,G=0.800000,B=0.000000,A=1.000000)" :NewEnumerator4 "(R=1.000000,G=1.000000,B=1.000000,A=1.000000)"))
  (Rendering|Material|SetMaterial (Variables|Default|GetStaticMesh) 0 (Utilities|Select :Index (Variables|Default|GetColor) :NewEnumerator0 "/Game/MyGame/Mech_Color/Materials/Mat_Blue.Mat_Blue" :NewEnumerator1 "/Game/MyGame/Mech_Color/Materials/Mat_Red.Mat_Red" :NewEnumerator2 "/Game/MyGame/Mech_Color/Materials/Mat_Yellow.Mat_Yellow" :NewEnumerator4 "/Game/UE5/FPWeapon/Materials/BaseMaterial.BaseMaterial"))
  (Effects|Components|ParticleSystem|SetColorParameter (Variables|Default|GetNGR_ColorDetector) "Color" _returnvalue)
  (Rendering|Components|Light|SetLightColor (Variables|Default|GetSpotLight) _returnvalue true)
  (CallFunction|CalculateHeight))

(fn CheckObjectinSight
  (params (other :type Actor%20Object%20Reference))
  (bind _output_get (LocalVariables|SetlocalOther other))
  (bind _outactors (Actor|GetAllActorswithTag (Variables|Default|GetDetectionNoBlockTag)))
  (Utilities|Array|Add _outactors (Variables|Default|GetparentPlatform))
  (bind _outhit (Collision|SphereTraceByChannel (Transformation|GetWorldLocation (Variables|Default|GetSphereTraceStartPoint)) (Transformation|GetWorldLocation (Variables|/Script/Engine.Actor|GetRootComponent _output_get)) 5e+01 "TraceTypeQuery1" false _outactors "None"))
  (return (== (.HitActor (Collision|BreakHitResult _outhit)) (LocalVariables|GetlocalOther))))

(fn CalculateHeight
  (bind _spotlight (Variables|Default|GetSpotLight))
  (bind _capsule (Variables|Default|GetCapsule))
  (bind _spheretracestartpoint (Variables|Default|GetSphereTraceStartPoint))
  (bind _returnvalue (Transformation|GetWorldLocation _spheretracestartpoint))
  (bind _outactors (Actor|GetAllActorsOfClass "/Game/MyGame/Mech_Color/Paintable/Cube/BP_PaintableCube.BP_PaintableCube_C"))
  (bind _outhit (Collision|LineTraceByChannel _returnvalue (+ _returnvalue (* (Math|Vector|GetForwardVector (Variables|Default|GetArrow)) 2e+03)) "TraceTypeQuery1" false _outactors "None"))
  (Effects|Components|ParticleSystem|SetFloatParameter (Variables|Default|GetNGR_ColorDetector) "Cylinder Height" (Math|Float|SelectFloat 2e+03 (.Distance (Collision|BreakHitResult _outhit)) (== (.Distance (Collision|BreakHitResult _outhit)) 0.0)))
  (Rendering|Lighting|SetAttenuationRadius _spotlight (Math|Float|SelectFloat 2e+03 (.Distance (Collision|BreakHitResult _outhit)) (== (.Distance (Collision|BreakHitResult _outhit)) 0.0)))
  (Rendering|Lighting|SetOuterConeAngle _spotlight (/ (Variables|Default|GetsizeMultiplier) (/ (Math|Float|SelectFloat 2e+03 (.Distance (Collision|BreakHitResult _outhit)) (== (.Distance (Collision|BreakHitResult _outhit)) 0.0)) 2e+02)))
  (Components|Capsule|SetCapsuleSize _capsule 1.5e+02 (/ (Math|Float|SelectFloat 2e+03 (.Distance (Collision|BreakHitResult _outhit)) (== (.Distance (Collision|BreakHitResult _outhit)) 0.0)) 2.0) true)
  (Transformation|SetRelativeLocation _capsule (Math|Vector|MakeVector 0.0 0.0 (Math|Float|SelectFloat 2e+03 (.Distance (Collision|BreakHitResult _outhit)) (== (.Distance (Collision|BreakHitResult _outhit)) 0.0))) false false))