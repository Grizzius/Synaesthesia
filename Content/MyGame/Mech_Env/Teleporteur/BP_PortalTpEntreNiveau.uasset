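; Color-gated portal that teleports the first-person player to another level when its current color matches its required color.
; Overlapping the trigger box fades the screen, optionally writes a new progression state to GI_Main, then opens the target level.
; ChangeColor sets the current color, tinting the light and toggling its intensity and the portal effect on a match.
; The construction script tints the effect by the required color.
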(event OnComponentBeginOverlap(BoxTP)
  (params (OverlappedComponent :type Primitive%20Component%20Object%20Reference) (OtherActor :type Actor%20Object%20Reference) (OtherComp :type Primitive%20Component%20Object%20Reference) (OtherBodyIndex :type Integer) (bFromSweep :type Boolean) (SweepResult :type Hit%20Result%20Structure%20%28by%20ref%29))
  (bind _asbp_first_person (Utilities|Casting|CastToBP_FirstPerson OtherActor))
  (CallFunction|TeleportPlayer _asbp_first_person))

(event Custom|TeleportPlayer
  (params (Player :type BP%20First%20Person%20Object%20Reference))
  (if (Utilities|Enum|Equal(Enum) (Variables|Default|GetcolorCondition) (Variables|Default|Getcolor))
    (Default|EventFade (Variables|/Game/MyGame/Joueur/Character/BP_FirstPerson.BP_FirstPerson_C|GetMainMenu Player) false)
    (Utilities|FlowControl|Delay 1.0)
    (if (Variables|Default|GetbChangeProgressionState?)
      (bind _asgi_main (Utilities|Casting|CastToGI_Main (Game|GetGameInstance)))
      (Variables|/Game/MyGame/Data/GameInstance/GI_Main.GI_Main_C|SetProgressionState _asgi_main (Variables|Default|GetNewProgressionState)))
    (Game|OpenLevel(byObjectReference) (Variables|Default|GetLevel))
    (Audio|PlaySound2D "/Game/MyGame/Sound/SoundEffect/WAV/Unlock.Unlock" 1.0 1.0 0.0 0 0)))

(event EventBeginPlay)

(event Collision|EventActorBeginOverlap
  (params (OtherActor :type Actor%20Object%20Reference)))

(event EventTick
  (params (DeltaSeconds :type Float%20%28single-precision%29)))

(event EventChangeColor
  (params (newColor :type EnumColor%20Enum :default "NewEnumerator0"))
  (bind _e (Variables|Default|Gete))
  (bind _output_get (Variables|Default|Setcolor newColor))
  (Rendering|Components|Light|SetLightColor _e (Utilities|Select :Index _output_get :NewEnumerator0 "(R=0.000000,G=0.000000,B=1.000000,A=1.000000)" :NewEnumerator1 "(R=1.000000,G=0.000000,B=0.000000,A=1.000000)" :NewEnumerator2 "(R=1.000000,G=1.000000,B=0.000000,A=1.000000)" :NewEnumerator4 "") true)
  (Rendering|Components|Light|SetIntensity _e (Math|Float|SelectFloat 1e+04 1e+02 (Utilities|Enum|Equal(Enum) (Variables|Default|GetcolorCondition) (Variables|Default|Getcolor))))
  (Rendering|SetVisibility (Variables|Default|GetPortailSFX) (Utilities|Enum|Equal(Enum) (Variables|Default|GetcolorCondition) (Variables|Default|Getcolor)) false))

(event EventDisplayInteractHUD)

(event EventHideInteractHUD)

(fn ConstructionScript
  (Effects|Components|ParticleSystem|SetColorParameter (Variables|Default|GetPortailSFX) "Color" (Utilities|Select :Index (Variables|Default|GetcolorCondition) :NewEnumerator0 "(R=0.000000,G=0.000000,B=1.000000,A=1.000000)" :NewEnumerator1 "(R=1.000000,G=0.000000,B=0.000000,A=1.000000)" :NewEnumerator2 "(R=1.000000,G=1.000000,B=0.000000,A=1.000000)" :NewEnumerator4 "(R=1.000000,G=1.000000,B=1.000000,A=1.000000)"))
  (Rendering|SetVisibility (Variables|Default|GetPortailSFX) (Utilities|Enum|Equal(Enum) (Variables|Default|GetcolorCondition) (Variables|Default|Getcolor)) false))