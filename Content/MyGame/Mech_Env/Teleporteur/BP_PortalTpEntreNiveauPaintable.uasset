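; BP_PortalTpEntreNiveauPaintable is a paintable portal that teleports the first-person player to another level.
; ChangeColor stores the portal's color and tints its RectLight to match.
; Overlapping BoxTP while the current color equals the required color opens the target level and plays an unlock sound.
; Before loading, it can optionally write a new progression state to the GI_Main game instance.
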(event OnComponentBeginOverlap(BoxTP)
  (params (OverlappedComponent :type Primitive%20Component%20Object%20Reference) (OtherActor :type Actor%20Object%20Reference) (OtherComp :type Primitive%20Component%20Object%20Reference) (OtherBodyIndex :type Integer) (bFromSweep :type Boolean) (SweepResult :type Hit%20Result%20Structure%20%28by%20ref%29))
  (if (Utilities|Enum|Equal(Enum) (Variables|Default|GetCurrentColor) (Variables|Default|GetRequiredColor))
    (Utilities|Casting|CastToBP_FirstPerson OtherActor)
    (if (Variables|Default|GetbChangeProgressionState?)
      (bind _asgi_main (Utilities|Casting|CastToGI_Main (Game|GetGameInstance)))
      (Variables|/Game/MyGame/Data/GameInstance/GI_Main.GI_Main_C|SetProgressionState _asgi_main (Variables|Default|GetNewProgressionState)))
    (Game|OpenLevel(byObjectReference) (Variables|Default|GetLevel_0))
    (Audio|PlaySound2D "/Game/MyGame/Sound/SoundEffect/WAV/Unlock.Unlock" 1.0 1.0 0.0 0 0)))

(event EventBeginPlay)

(event Collision|EventActorBeginOverlap
  (params (OtherActor :type Actor%20Object%20Reference)))

(event EventTick
  (params (DeltaSeconds :type Float%20%28single-precision%29)))

(event EventChangeColor
  (params (newColor :type EnumColor%20Enum :default "NewEnumerator0"))
  (bind _output_get (Variables|Default|SetCurrentColor newColor))
  (Rendering|Components|Light|SetLightColor (Variables|Default|GetRectLight) (Utilities|Select :Index _output_get :NewEnumerator0 "(R=0.000000,G=0.000000,B=1.000000,A=1.000000)" :NewEnumerator1 "(R=1.000000,G=0.000000,B=0.000000,A=1.000000)" :NewEnumerator2 "(R=1.000000,G=1.000000,B=0.000000,A=1.000000)" :NewEnumerator4 "(R=1.000000,G=1.000000,B=1.000000,A=1.000000)") true))

(fn ConstructionScript)